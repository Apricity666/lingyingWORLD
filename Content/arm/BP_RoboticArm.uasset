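; Robotic arm actor that moves a static mesh to follow a location held in the arm's animation Blueprint.
; Each tick it looks up a BP_RoboticArm in the level, casts its anim instance to ABP_RoboticArm and reads the Full transform's location.
; That location is axis-swapped, scaled by 100 and shifted by fixed offsets into the mesh's world position.
; Disconnected nodes for converting mesh position back are unused.
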(event `self.ReceiveTick`
  (params (DeltaSeconds :type "Float (single-precision)"))
  (bind _returnvalue (`GameplayStatics.GetActorOfClass` "BP_RoboticArm_C"))
  (bind _asabp_robotic_arm (cast `/Game/arm/ABP_RoboticArm` (`SkeletalMeshComponent.GetAnimInstance` (`/Game/arm/BP_RoboticArm.RoboticArm` _returnvalue))))
  (bind _full (`/Game/arm/ABP_RoboticArm.Full` _asabp_robotic_arm))
  (`SceneComponent.K2_SetWorldLocation` (`self.StaticMesh`) (`KismetMathLibrary.MakeVector` (+ (* (.z (.location _full)) 100.0) 176.0) (+ (* (.x (.location _full)) 100.0) 47.0) (+ (* (.y (.location _full)) 100.0) 182.0)) false false))

(fn `UserConstructionScript`)